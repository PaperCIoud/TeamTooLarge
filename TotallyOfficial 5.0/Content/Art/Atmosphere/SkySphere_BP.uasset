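; Sky sphere actor that sets a level's sun, sky gradient, stars, color tinting and four-layer fog from its variables.
; The construction script creates a dynamic sky material and drives it alongside the directional light, sharing color and rotation-derived direction.
; Tint and fog values go to the PP_parameters material parameter collection, on construction and again at BeginPlay.
; A separate landscape tint function writes to that collection but is not called here.
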(event EventBeginPlay
  (CallFunction|UpdateShader)
  (CallFunction|UpdateFog))

(fn ConstructionScript
  (bind _returnvalue (Rendering|Material|CreateDynamicMaterialInstance (Variables|Default|GetSphereSky) 0 "/Game/Art/Materials/Sky.Sky" "None" :!class /Script/Engine.PrimitiveComponent))
  (Variables|Default|SetSky%20Material _returnvalue)
  (CallFunction|UpdateLightSource)
  (CallFunction|UpdateSky)
  (CallFunction|UpdateStars)
  (CallFunction|UpdateShader)
  (CallFunction|UpdateFog))

(fn UpdateLightSource
  (bind _light_source_height (Variables|LightSource|GetLight%20Source%20Height))
  (bind _light_source_rotation (Variables|LightSource|GetLight%20Source%20Rotation))
  (bind _sky_material (Variables|Default|GetSky%20Material))
  (bind _light_source_color (Variables|LightSource|GetLight%20Source%20Color))
  (bind _returnvalue (- 3.6e+02 _light_source_height))
  (bind _returnvalue_2 (Math|Rotator|MakeRotator 0.0 _returnvalue _light_source_rotation))
  (Rendering|Components|Light|SetLightColor (Variables|Default|GetDirectionalLight) _light_source_color true)
  (Rendering|Material|SetVectorParameterValue (Variables|Default|GetSky%20Material) "Sun color" _light_source_color :!class /Script/Engine.MaterialInstanceDynamic)
  (Transformation|SetRelativeRotation (Variables|Default|GetDirectionalLight) _returnvalue_2 false false)
  (Rendering|Material|SetVectorParameterValue (Variables|Default|GetSky%20Material) "Light direction" (Math|Conversions|ToLinearColor(Vector) (Math|Rotator|GetRotationXVector _returnvalue_2)) :!class /Script/Engine.MaterialInstanceDynamic)
  (Rendering|Material|SetScalarParameterValue _sky_material "Sun Radius" (Variables|LightSource|GetLight%20Disc%20Size) :!class /Script/Engine.MaterialInstanceDynamic)
  (Rendering|Material|SetScalarParameterValue _sky_material "Sun brightness" (Variables|LightSource|GetLight%20Disc%20Brightness) :!class /Script/Engine.MaterialInstanceDynamic)
  (Rendering|Components|Light|SetIntensity (Variables|Default|GetDirectionalLight) (Variables|LightSource|GetLight%20Source%20Intensity)))

(fn UpdateSky
  (Rendering|Material|SetVectorParameterValue (Variables|Default|GetSky%20Material) "Sky Bottom Color" (Variables|Sky|GetHorizon%20Color) :!class /Script/Engine.MaterialInstanceDynamic)
  (Rendering|Material|SetVectorParameterValue (Variables|Default|GetSky%20Material) "Sky Top Color" (Variables|Sky|GetSky%20Color) :!class /Script/Engine.MaterialInstanceDynamic)
  (Rendering|Material|SetScalarParameterValue (Variables|Default|GetSky%20Material) "Sky Bottom Threshold" (Variables|Sky|GetHorizon%20Threshold) :!class /Script/Engine.MaterialInstanceDynamic)
  (Rendering|Material|SetScalarParameterValue (Variables|Default|GetSky%20Material) "Sky Top Threshold" (Variables|Sky|GetSky%20Threshold) :!class /Script/Engine.MaterialInstanceDynamic))

(fn UpdateStars
  (Rendering|Material|SetScalarParameterValue (Variables|Default|GetSky%20Material) "Star brightness" (Variables|Stars|GetStar%20Brightness) :!class /Script/Engine.MaterialInstanceDynamic)
  (Rendering|Material|SetVectorParameterValue (Variables|Default|GetSky%20Material) "Star Color" (Variables|Stars|GetStar%20Color) :!class /Script/Engine.MaterialInstanceDynamic))

(fn UpdateShader
  (Rendering|Material|SetVectorParameterValue "/Game/Art/Atmosphere/PP_parameters.PP_parameters" "Light Area Tint" (Variables|Shader|GetLight%20Area%20Tint) :!class /Script/Engine.KismetMaterialLibrary)
  (Rendering|Material|SetVectorParameterValue "/Game/Art/Atmosphere/PP_parameters.PP_parameters" "Dark Area Tint" (Variables|Shader|GetDark%20Area%20Tint) :!class /Script/Engine.KismetMaterialLibrary)
  (Rendering|Material|SetScalarParameterValue "/Game/Art/Atmosphere/PP_parameters.PP_parameters" "Light Blend Amount" (Variables|Shader|GetLight%20Blend%20Amount) :!class /Script/Engine.KismetMaterialLibrary)
  (Rendering|Material|SetScalarParameterValue "/Game/Art/Atmosphere/PP_parameters.PP_parameters" "Dark Blend Amount" (Variables|Shader|GetDark%20Blend%20Amount) :!class /Script/Engine.KismetMaterialLibrary)
  (Rendering|Material|SetScalarParameterValue "/Game/Art/Atmosphere/PP_parameters.PP_parameters" "Darkness Factor" (Variables|Shader|GetDarkness%20Threshold) :!class /Script/Engine.KismetMaterialLibrary))

(fn UpdateFog
  (Rendering|Material|SetVectorParameterValue "/Game/Art/Atmosphere/PP_parameters.PP_parameters" "Fog Color 1" (Variables|Fog|GetFog%20Color%201) :!class /Script/Engine.KismetMaterialLibrary)
  (Rendering|Material|SetVectorParameterValue "/Game/Art/Atmosphere/PP_parameters.PP_parameters" "Fog Color 2" (Variables|Fog|GetFog%20Color%202) :!class /Script/Engine.KismetMaterialLibrary)
  (Rendering|Material|SetVectorParameterValue "/Game/Art/Atmosphere/PP_parameters.PP_parameters" "Fog Color 3" (Variables|Fog|GetFog%20Color%203) :!class /Script/Engine.KismetMaterialLibrary)
  (Rendering|Material|SetVectorParameterValue "/Game/Art/Atmosphere/PP_parameters.PP_parameters" "Fog Color 4" (Variables|Fog|GetFog%20Color%204) :!class /Script/Engine.KismetMaterialLibrary)
  (Rendering|Material|SetScalarParameterValue "/Game/Art/Atmosphere/PP_parameters.PP_parameters" "Fog Distance 1" (Variables|Fog|GetFog%20Distance%201) :!class /Script/Engine.KismetMaterialLibrary)
  (Rendering|Material|SetScalarParameterValue "/Game/Art/Atmosphere/PP_parameters.PP_parameters" "Fog Distance 2" (Variables|Fog|GetFog%20Distance%202) :!class /Script/Engine.KismetMaterialLibrary)
  (Rendering|Material|SetScalarParameterValue "/Game/Art/Atmosphere/PP_parameters.PP_parameters" "Fog Distance 3" (Variables|Fog|GetFog%20Distance%203) :!class /Script/Engine.KismetMaterialLibrary)
  (Rendering|Material|SetScalarParameterValue "/Game/Art/Atmosphere/PP_parameters.PP_parameters" "Fog Distance 4" (Variables|Fog|GetFog%20Distance%204) :!class /Script/Engine.KismetMaterialLibrary)
  (Rendering|Material|SetScalarParameterValue "/Game/Art/Atmosphere/PP_parameters.PP_parameters" "Fog Opacity" (Variables|Fog|GetFog%20Opacity) :!class /Script/Engine.KismetMaterialLibrary)
  (Rendering|Material|SetScalarParameterValue "/Game/Art/Atmosphere/PP_parameters.PP_parameters" "Fog Opacity 1" (Variables|Fog|GetFog%20Opacity%201) :!class /Script/Engine.KismetMaterialLibrary)
  (Rendering|Material|SetScalarParameterValue "/Game/Art/Atmosphere/PP_parameters.PP_parameters" "Fog Opacity 2" (Variables|Fog|GetFog%20Opacity%202) :!class /Script/Engine.KismetMaterialLibrary)
  (Rendering|Material|SetScalarParameterValue "/Game/Art/Atmosphere/PP_parameters.PP_parameters" "Fog Opacity 3" (Variables|Fog|GetFog%20Opacity%203) :!class /Script/Engine.KismetMaterialLibrary)
  (Rendering|Material|SetScalarParameterValue "/Game/Art/Atmosphere/PP_parameters.PP_parameters" "Fog Opacity 4" (Variables|Fog|GetFog%20Opacity%204) :!class /Script/Engine.KismetMaterialLibrary))

(fn UpdateLandscapeShader
  (Rendering|Material|SetVectorParameterValue "/Game/Art/Atmosphere/PP_parameters.PP_parameters" "Light Area Tint 1" (Variables|LandscapeShader|GetLight%20Area%20Tint%20Landscape) :!class /Script/Engine.KismetMaterialLibrary)
  (Rendering|Material|SetVectorParameterValue "/Game/Art/Atmosphere/PP_parameters.PP_parameters" "Dark Area Tint 1" (Variables|LandscapeShader|GetDark%20Area%20Tint%20Landscape) :!class /Script/Engine.KismetMaterialLibrary)
  (Rendering|Material|SetScalarParameterValue "/Game/Art/Atmosphere/PP_parameters.PP_parameters" "Light Blend Amount 1" (Variables|LandscapeShader|GetLight%20Blend%20Amount%20Landscape) :!class /Script/Engine.KismetMaterialLibrary)
  (Rendering|Material|SetScalarParameterValue "/Game/Art/Atmosphere/PP_parameters.PP_parameters" "Dark Blend Amount 1" (Variables|LandscapeShader|GetDark%20Blend%20Amount%20Landscape) :!class /Script/Engine.KismetMaterialLibrary)
  (Rendering|Material|SetScalarParameterValue "/Game/Art/Atmosphere/PP_parameters.PP_parameters" "Darkness Factor 1" (Variables|LandscapeShader|GetDarkness%20Threshold%20Landscape) :!class /Script/Engine.KismetMaterialLibrary))