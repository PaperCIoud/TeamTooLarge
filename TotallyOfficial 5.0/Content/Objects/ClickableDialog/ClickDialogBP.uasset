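; Interactable world object that plays a click-through dialog with optional voice audio, selected by its DialogID.
; BeginPlay caches matching DialogTest row names, and GetLine looks up the current LineNumber among them.
; Interact opens the dialog widget in UI-only input; each click advances text and audio, and empty text closes it and resets.
; Tick shows a camera-facing interact prompt while the player is near.
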(event Custom|OnClick_Event_0
  (bind _returnvalue (Game|GetPlayerController 0))
  ;[1 1 1] Show/Close dialog widget
  (Math|Integer|IncrementInt (Variables|Default|GetlineNumber)
    (:%20%20
      (bind (_currentline _currentlineaudio) (CallFunction|GetLine))
      (if (!= (Class|KismetTextLibrary|GetEmptyText) _currentline)
        (Variables|Default|SetCurrent%20Line%20Audio _currentlineaudio)
        (Variables|/Game/Objects/ClickableDialog/ClickDialogWidget.ClickDialogWidget_C|SetdialogText (Variables|Default|GetClickDialogWidget) _currentline)
        ;;[1 1 1] Dialog Audio Management
        (Utilities|IsValid (Variables|Default|GetCurrent%20Line%20Audio)
          (:Is%20Valid
            (Utilities|IsValid (Variables|Default|Getsound)
              (:Is%20Valid
                (if (Audio|Components|Audio|IsPlaying (Variables|Default|Getsound))
                  (Audio|Components|Audio|Stop (Variables|Default|Getsound))))
              (:Is%20Not%20Valid
                _))
            (bind _returnvalue_2 (Audio|SpawnSoundatLocation (Variables|Default|GetCurrent%20Line%20Audio) (Transformation|GetActorLocation (Game|GetPlayerController 0)) "0, 0, 0" 1.0 1.0 0.0 0 0 false))
            (Audio|Components|Audio|Play _returnvalue_2 0.0)
            (Variables|Default|Setsound _returnvalue_2)))
        (else
          ;;[1 1 1] Remove widget and reset
          (Widget|RemovefromParent (Variables|Default|GetClickDialogWidget))
          (Utilities|IsValid (Variables|Default|Getsound)
            (:Is%20Valid
              (Audio|Components|Audio|Stop (Variables|Default|Getsound)))
            (:Is%20Not%20Valid
              _))
          (Variables|Default|SetlineNumber 1)
          (Variables|Default|SetClickDialogWidget 0)
          (Input|SetInputModeGameOnly _returnvalue)
          (Variables|/Script/Engine.PlayerController|SetbShowMouseCursor _returnvalue false))))))

(event EventBeginPlay
  ;[1 1 1] Grab Dialog
  (bind _outrownames (DataTable|GetDataTableRowNames "/Game/Objects/DialogTest.DialogTest"))
  (for _array_element _outrownames
    (bind _returnvalue (Utilities|GetDataTableRow "/Game/Objects/DialogTest.DialogTest" _array_element)
      (:then
        (if (== (.DialogID (Utilities|Struct|BreakDialogData _returnvalue)) (Variables|Default|GetdialogID))
          (Utilities|Array|Add (Variables|Default|GetthisDialog) _array_element))))))

(event EventTick
  (params (DeltaSeconds :type Float%20%28single-precision%29))
  (bind _presse (Variables|Default|GetPressE))
  ;[1 1 1] Show Interact Prompt
  (if (<= (Math|Vector|VectorLength (- (Transformation|GetActorLocation (Game|GetPlayerCharacter 0)) (Transformation|GetActorLocation))) 2e+02)
    (Rendering|SetVisibility _presse true false)
    (Transformation|SetWorldRotation (Variables|Default|GetPressE) (Math|Rotator|FindLookatRotation (Transformation|GetActorLocation) (Transformation|GetWorldLocation (Variables|/Script/Engine.PlayerCameraManager|GetTransformComponent (Game|GetPlayerCameraManager 0)))) false false)
    (else
      (Rendering|SetVisibility _presse false false))))

(event EventInteract
  (params (PlayerCharacter :type Third%20Person%20Character%20Object%20Reference))
  (bind _returnvalue (Game|GetPlayerController 0))
  ;[1 1 1] Show/Close dialog widget
  (Utilities|IsValid (Variables|Default|GetClickDialogWidget)
    (:Is%20Not%20Valid
      (bind _returnvalue_2 (UserInterface|CreateWidget "/Game/Objects/ClickableDialog/ClickDialogWidget.ClickDialogWidget_C" (Game|GetPlayerController 0)))
      (bind _output_get (Variables|Default|SetClickDialogWidget _returnvalue_2))
      (EventDispatchers|AssignOnClick _output_get (delegate Custom|OnClick_Event_0))
      (UserInterface|Viewport|AddtoViewport _output_get 0)
      (Input|SetInputModeUIOnly _returnvalue 0 "DoNotLock")
      (Variables|/Script/Engine.PlayerController|SetbShowMouseCursor _returnvalue true)
      (bind (_currentline _currentlineaudio) (CallFunction|GetLine))
      (Variables|/Game/Objects/ClickableDialog/ClickDialogWidget.ClickDialogWidget_C|SetdialogText (Variables|Default|GetClickDialogWidget) _currentline)
      (Utilities|IsValid _currentlineaudio
        (:Is%20Valid
          (bind _returnvalue_3 (Audio|SpawnSoundatLocation _currentlineaudio (Transformation|GetActorLocation (Game|GetPlayerController 0)) "0, 0, 0" 1.0 1.0 0.0 0 0 false))
          (Audio|Components|Audio|Play _returnvalue_3 0.0)
          (Variables|Default|Setsound _returnvalue_3))))))

(fn ConstructionScript
  (Rendering|Components|TextRender|SetText (Variables|Default|GetPressE) (Variables|Default|GetinteractPrompt)))

(fn GetLine
  (for _array_element (Variables|Default|GetthisDialog)
    (bind _returnvalue (Utilities|GetDataTableRow "/Game/Objects/DialogTest.DialogTest" _array_element)
      (:then
        (if (== (.LineID (Utilities|Struct|BreakDialogData _returnvalue)) (Variables|Default|GetlineNumber))
          (LocalVariables|SetcurrentDialog (.Dialog (Utilities|Struct|BreakDialogData _returnvalue)))
          (LocalVariables|SetcurrentDialogAudio (.Audio (Utilities|Struct|BreakDialogData _returnvalue)))))))
  (return (LocalVariables|GetcurrentDialog) (LocalVariables|GetcurrentDialogAudio)))