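; Gate actor that swings open and carries an attached readable paper note.
; The construction script configures the child PaperNotesBP with its prompt, text, mesh, paper sound and a reference back to this gate.
; OpenGate sets Opened and plays a timeline that drives EdgeCube's yaw, with a DoOnce limiting the stone gate sound to a single play.
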(event Custom|OpenGate
  (Variables|Default|Setopened true)
  (bind _openevent (Timeline|Open PlayFromStart)
    (:Update
      (Transformation|SetRelativeRotation (Variables|Default|Getedge_cube) (Math|Rotator|MakeRotator -9e+01 0.0 _openevent) false false)
      (Utilities|FlowControl|DoOnce false
        (:Completed
          (Audio|PlaySoundatLocation "/Game/Audio/SFX/SFX_stoneGate.SFX_stoneGate" (Transformation|GetWorldLocation (Variables|Default|GetDefaultSceneRoot)) "0, 0, 0" 1.0 1.0 0.0 0 0 0))))))

(event EventBeginPlay)

(event Collision|EventActorBeginOverlap
  (params (OtherActor :type Actor%20Object%20Reference)))

(event EventTick
  (params (DeltaSeconds :type Float%20%28single-precision%29)))

(fn ConstructionScript
  (bind _aspaper_notes_bp (Utilities|Casting|CastToPaperNotesBP (Variables|/Script/Engine.ChildActorComponent|GetChildActor (Variables|Default|GetPaperNotesBP))))
  (bind _output_get (Variables|Default|SetnoteAttached _aspaper_notes_bp))
  (Variables|/Game/Objects/MapNotes/PaperNotesBP.PaperNotesBP_C|SetpromptText _output_get "Read Note")
  (Variables|/Game/Objects/MapNotes/PaperNotesBP.PaperNotesBP_C|SetgateRef _output_get self)
  (Variables|/Game/Objects/MapNotes/PaperNotesBP.PaperNotesBP_C|SetnoteOpenSFX _output_get "/Game/Audio/SFX/SFX_paper.SFX_paper")
  (Variables|/Game/Objects/MapNotes/PaperNotesBP.PaperNotesBP_C|SetnoteText _output_get (Variables|Default|GetNote%20Text))
  (Variables|/Game/Objects/MapNotes/PaperNotesBP.PaperNotesBP_C|SetnoteMesh _output_get (Variables|Default|GetNote%20Mesh)))