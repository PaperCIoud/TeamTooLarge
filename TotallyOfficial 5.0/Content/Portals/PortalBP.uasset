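; Portal actor that teleports the third-person character to its paired portal's exit, defaulting to itself when unpaired.
; It starts inactive and stays hidden until active; Entrance overlap then moves the player, zeroing roll and aligning control rotation.
; A Fade volume adds a screen widget and opens a Tick gate, raising image opacity as local-Y distance shrinks.
; The construction script places Entrance and exit reference from variables.
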(event OnComponentBeginOverlap(entrance)
  (params (OverlappedComponent :type Primitive%20Component%20Object%20Reference) (OtherActor :type Actor%20Object%20Reference) (OtherComp :type Primitive%20Component%20Object%20Reference) (OtherBodyIndex :type Integer) (bFromSweep :type Boolean) (SweepResult :type Hit%20Result%20Structure%20%28by%20ref%29))
  (bind _pairedportal (Variables|Default|GetpairedPortal))
  (bind _exitref (Variables|PortalBP_C|GetexitRef _pairedportal))
  (bind _returnvalue (Transformation|GetWorldTransform _exitref))
  (bind (_roll _pitch _yaw) (Math|Rotator|BreakRotator (.rotation _returnvalue)))
  ;[1 1 1] Teleport on collision
  (bind _asthird_person_character (Utilities|Casting|CastToThirdPersonCharacter OtherActor))
  (bind _output_get (Variables|Default|Setplayer _asthird_person_character))
  (if (Variables|Default|GetisActive)
    (Transformation|SetActorTransform _output_get (Math|Transform|MakeTransform (.location _returnvalue) (Math|Rotator|MakeRotator 0.0 _pitch _yaw) "1,1,1"))
    (Pawn|SetControlRotation (Game|GetPlayerController 0) (Transformation|GetActorRotation (Variables|Default|Getplayer)))))

(event OnComponentBeginOverlap(fade)
  (params (OverlappedComponent :type Primitive%20Component%20Object%20Reference) (OtherActor :type Actor%20Object%20Reference) (OtherComp :type Primitive%20Component%20Object%20Reference) (OtherBodyIndex :type Integer) (bFromSweep :type Boolean) (SweepResult :type Hit%20Result%20Structure%20%28by%20ref%29))
  (bind _self self)
  (bind _returnvalue (Transformation|GetActorTransform _self))
  (bind (_location _rotation) (Math|Transform|BreakTransform _returnvalue))
  ;[1 1 1] Fade Opacity
  (Utilities|Casting|CastToThirdPersonCharacter OtherActor)
  (Utilities|Casting|CastToCapsuleComponent OtherComp)
  (if (Variables|Default|GetisActive)
    (bind _returnvalue_2 (UserInterface|CreateWidget "/Game/Portals/PortalFadeWidget.PortalFadeWidget_C"))
    (bind _output_get (Variables|Default|SetfadeWidget _returnvalue_2))
    (UserInterface|Viewport|AddtoViewport _output_get 0)
    (Utilities|FlowControl|Gate true) ; enters at Open
  ))

(event OnComponentEndOverlap(fade)
  (params (OverlappedComponent :type Primitive%20Component%20Object%20Reference) (OtherActor :type Actor%20Object%20Reference) (OtherComp :type Primitive%20Component%20Object%20Reference) (OtherBodyIndex :type Integer))
  (bind _self self)
  (bind _returnvalue (Transformation|GetActorTransform _self))
  (bind (_location _rotation) (Math|Transform|BreakTransform _returnvalue))
  ;[1 1 1] Fade Opacity
  (Utilities|Casting|CastToThirdPersonCharacter OtherActor)
  (Utilities|Casting|CastToCapsuleComponent OtherComp)
  (if (Variables|Default|GetisActive)
    (Widget|RemovefromParent (Variables|Default|GetfadeWidget))
    (Utilities|FlowControl|Gate true) ; enters at Close
  ))

(event EventBeginPlay
  ;[1 1 1] Set Default Values
  (Variables|Default|SetisActive false)
  (if (not (Utilities|IsValid (Variables|Default|GetpairedPortal)))
    (Variables|Default|SetpairedPortal self)))

(event EventTick
  (params (DeltaSeconds :type Float%20%28single-precision%29))
  (bind _self self)
  (bind _returnvalue (Transformation|GetActorTransform _self))
  (bind (_location _rotation) (Math|Transform|BreakTransform _returnvalue))
  ;[1 1 1] Fade Opacity
  (Rendering|SetActorHiddenInGame (not (Variables|Default|GetisActive)))
  (Utilities|FlowControl|Gate true
    (:Exit
      (Class|Image|SetOpacity (Variables|/Game/Portals/PortalFadeWidget.PortalFadeWidget_C|GetbackImage (Variables|Default|GetfadeWidget)) (- 1.0 (Math|Float|Clamp(Float) (/ (- (Math|Float|Absolute(Float) (- (.Y (Math|Vector|BreakVector (Math|Vector|RotateVector (- (.Location (Math|Transform|BreakTransform (Transformation|GetActorTransform (Game|GetPlayerCharacter 0)))) _location) (Class|KismetMathLibrary|NegateRotator _rotation)))) 59.0)) 141.0) 901.0)))))))

(fn ConstructionScript
  (Transformation|SetRelativeTransform (Variables|Default|Getentrance) (Variables|Default|GetentranceTransform) false false)
  (Transformation|SetRelativeLocation (Variables|Default|GetexitRef) (Variables|Default|GetexitLocation) false false))