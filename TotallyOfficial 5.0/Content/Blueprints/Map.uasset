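; Map actor that switches the visibility of staged static mesh groups, tagged map1 to map3.
; UpdateMap takes a stage number and toggles the matching tagged components without propagating to children, so repeat calls flip them back.
; The construction script toggles the first stage, and releasing V toggles the second.
; The third stage is handled but not called within this Blueprint.
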(event EventBeginPlay)

(event Collision|EventActorBeginOverlap
  (params (OtherActor :type Actor%20Object%20Reference)))

(event EventTick
  (params (DeltaSeconds :type Float%20%28single-precision%29)))

(event Input|KeyboardEvents|V
  (params (Key :type Key%20Structure :default "None"))
  (:Released
    (CallFunction|UpdateMap 2)))

(fn ConstructionScript
  (CallFunction|UpdateMap 1))

(fn UpdateMap
  (params (Stage :type Integer))
  (switch int Stage
    (:1
      (Rendering|ToggleVisibility (Actor|GetComponentsbyTag "/Script/Engine.StaticMeshComponent" "map1") false))
    (:2
      (Rendering|ToggleVisibility (Actor|GetComponentsbyTag "/Script/Engine.StaticMeshComponent" "map2") false))
    (:3
      (Rendering|ToggleVisibility (Actor|GetComponentsbyTag "/Script/Engine.StaticMeshComponent" "map3") false))))